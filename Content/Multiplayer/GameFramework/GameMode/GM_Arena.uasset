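; Arena multiplayer game mode that chooses which pawn class each player controller spawns with.
; It overrides GetDefaultPawnClassForController, casting to PC_Base and looking up its character type in the PlayersClass map.
; Players whose info marks the character as dead get BP_ResurrectionFlowe instead, and an unset character type falls back to the parent's default.
; BeginPlay, Tick and the Test event are empty.
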(event Custom|Test
  (params (NewParam :type PC%20Base%20Object%20Reference)))

(event EventBeginPlay)

(event EventTick
  (params (DeltaSeconds :type Float%20%28single-precision%29)))

(fn ConstructionScript)

(fn GetDefaultPawnClassforController
  (params (InController :type Controller%20Object%20Reference))
  (bind _returnvalue (|CallParentFunction InController))
  (bind _aspc_base (Utilities|Casting|CastToPC_Base InController))
  (if (Utilities|Enum|NotEqual(Enum) (Variables|/Script/Multiplayer.MPlayerController|GetTypeOfCharacter _aspc_base) "None")
    (bind _returnvalue_2 (Class|MPlayerController|GetPlayerInfo _aspc_base))
    (if (.bCharacterDeath (Utilities|Struct|BreakPlayerInfoStruct _returnvalue_2))
      (return "/Game/Multiplayer/AdditionalActor/BP_ResurrectionFlowe.BP_ResurrectionFlowe_C")
      (else
        (return (.Value (Utilities|Map|Find (Variables|Default|GetPlayersClass) (Variables|/Script/Multiplayer.MPlayerController|GetTypeOfCharacter _aspc_base))))))
    (else
      (return _returnvalue))))